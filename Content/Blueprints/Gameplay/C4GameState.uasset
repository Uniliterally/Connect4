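; Game state for a two-player Connect Four match, holding the board as an array of columns along with turn and winner.
; An authority-only Tick drives the waiting, in-game and win-screen states, assigning tokens, resetting the board and restarting after a countdown.
; AddTokenToColumn fills the first empty slot, then either ends the round or swaps turns.
; Win checks test the placed token's column and row, and walk outward along both diagonals.
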(event EventTick
  (params (DeltaSeconds :type Float%20%28single-precision%29))
  (bind _playerarray (Variables|Default|GetPlayerArray))
  (bind _returnvalue (Utilities|Array|Length _playerarray))
  (bind _returnvalue_2 (>= _returnvalue 2))
  (Networking|SwitchHasAuthority
    (:Authority
      (switch Utilities|FlowControl|Switch|SwitchonPlayState (Variables|Default|GetPlay%20State)
        (:NewEnumerator0
          (if _returnvalue_2
            (Variables|Default|SetPlay%20State "NewEnumerator1" :!label _label)
            (Variables|Default|SetCurrent%20Turn "NewEnumerator1")
            (for (_array_element _array_index) _playerarray
              (bind _asc4player_state (Utilities|Casting|CastToC4PlayerState _array_element))
              (Variables|/Game/Blueprints/Gameplay/C4PlayerState.C4PlayerState_C|SetAssigned%20Token _asc4player_state (Utilities|Select :Index _array_index :Option%200 "NewEnumerator1" :Option%201 "NewEnumerator2"))
              (CallFunction|ResetBoard))))
        (:NewEnumerator1
          (if (not _returnvalue_2)
            (Variables|Default|SetPlay%20State "NewEnumerator0")))
        (:NewEnumerator2
          (bind _output_get (Variables|Default|SetCountdown (- (Variables|Default|GetCountdown) DeltaSeconds)))
          (if (<= _output_get 0.0)
            (goto _label)))))))

(fn ConstructionScript)

(fn GetTokenatPosition
  (params (Column :type Integer) (Row :type Integer))
  ;[1 1 1] Check we're looking in range
  (if (Math|Boolean|ORBoolean (< Column 0) (< Row 0) (>= Column 7))
    (return "NewEnumerator0")
    (else
      (return (Utilities|Array|Get(acopy) (Utilities|Struct|BreakColumnStruct (Utilities|Array|Get(acopy) (Variables|Default|GetBoard%20State) Column)) Row)))))

(fn AddTokentoColumn
  (params (Column :type Integer) (Token :type TokenType%20Enum :default "NewEnumerator0"))
  (bind _board_state (Variables|Default|GetBoard%20State))
  (bind _output (Utilities|Array|Get(acopy) _board_state Column))
  (bind _contents (Utilities|Struct|BreakColumnStruct _output))
  (for (_array_element _array_index) _contents
    (if (Utilities|Enum|Equal(Enum) _array_element "NewEnumerator0")
      (Utilities|Array|SetArrayElem _contents _array_index Token)
      (bind _win (CallFunction|CheckforWin Column _array_index))
      (if _win
        (Variables|Default|SetPlay%20State "NewEnumerator2")
        (Variables|Default|SetWinner (Variables|Default|GetCurrent%20Turn))
        (Variables|Default|SetCurrent%20Turn "NewEnumerator0")
        (Variables|Default|SetCountdown 5.0)
        (else
          (Variables|Default|SetCurrent%20Turn (select (Utilities|Enum|Equal(Enum) (Variables|Default|GetCurrent%20Turn) "NewEnumerator1") "NewEnumerator2" "NewEnumerator1"))))
      (return true)))
  (return false))

(fn ResetBoard
  (bind _board_state (Variables|Default|GetBoard%20State))
  (for _index (range 0 (- (Utilities|Array|Length _board_state) 1))
    (for (_ _array_index) (Utilities|Struct|BreakColumnStruct (Utilities|Array|Get(acopy) _board_state _index))
      (Utilities|Array|SetArrayElem (Utilities|Struct|BreakColumnStruct (Utilities|Array|Get(acopy) _board_state _index)) _array_index "NewEnumerator0"))))

(fn CheckforWin
  (params (Column :type Integer) (Row :type Integer))
  (Utilities|FlowControl|Sequence
    (:then_0
      (bind _win (CallFunction|WinCheckColumn Column))
      (if _win
        (return true)))
    (:then_1
      (bind _win_2 (CallFunction|WinCheckRow Row))
      (if _win_2
        (return true)))
    (:then_2
      (bind _win_3 (CallFunction|WinCheckDiagonal Column Row))
      (if _win_3
        (return true)))
    (:then_3
      (return false))))

(fn WinCheckColumn
  (params (Column :type Integer))
  (for _array_element (Utilities|Struct|BreakColumnStruct (Utilities|Array|Get(acopy) (Variables|Default|GetBoard%20State) Column))
    (if (Utilities|Enum|Equal(Enum) _array_element (Variables|Default|GetCurrent%20Turn))
      (Math|Integer|IncrementInt (LocalVariables|GetCount)
        (:%20%20
          (if (>= (LocalVariables|GetCount) 4)
            (return true))))
      (else
        (LocalVariables|SetCount 0))))
  (return false))

(fn WinCheckRow
  (params (Row :type Integer))
  (for _array_element (Variables|Default|GetBoard%20State)
    (if (Utilities|Enum|Equal(Enum) (Utilities|Array|Get(acopy) (Utilities|Struct|BreakColumnStruct _array_element) Row) (Variables|Default|GetCurrent%20Turn))
      (Math|Integer|IncrementInt (LocalVariables|GetCount)
        (:%20%20
          (if (>= (LocalVariables|GetCount) 4)
            (return true))))
      (else
        (LocalVariables|SetCount 0))))
  (return false))

(fn WinCheckDiagonal
  (params (Column :type Integer) (Row :type Integer))
  (Utilities|FlowControl|Sequence
    (:then_0
      (bind _out (CallFunction|CountDiagonal Column Row -1 -1))
      (LocalVariables|SetCount _out)
      (bind _out_2 (CallFunction|CountDiagonal Column Row 1 1))
      (LocalVariables|SetCount (+ (LocalVariables|GetCount) _out_2)))
    (:then_1
      (bind _out_3 (CallFunction|CountDiagonal Column Row -1 1))
      (LocalVariables|SetCount _out_3)
      (bind _out_4 (CallFunction|CountDiagonal Column Row 1 -1))
      (LocalVariables|SetCount (+ (LocalVariables|GetCount) _out_4)))
    (:then_2
      (return false)))
  ;[1 1 1] First token is counted twice
  (bind _result (Math|Integer|DecrementInt (LocalVariables|GetCount))
    (:%20%20
      (if (>= _result 4)
        (return true)))))

(fn CountDiagonal
  (params (Column :type Integer) (Row :type Integer) (Column%20Offset :type Integer) (Row%20Offset :type Integer))
  (bind _count (LocalVariables|GetCount))
  (bind _count_2 (LocalVariables|GetCount))
  (bind (_column_adjusted _row_adjusted) (Utilities|MakeAdjustment Column Row Column%20Offset Row%20Offset _count_2))
  (bind (_column_adjusted_2 _row_adjusted_2) (Utilities|MakeAdjustment Column Row Column%20Offset Row%20Offset _count))
  (bind _token (CallFunction|GetTokenatPosition _column_adjusted_2 _row_adjusted_2))
  (LocalVariables|SetCurrent%20Token _token)
  (while (Utilities|Enum|Equal(Enum) (Variables|Default|GetCurrent%20Turn) (LocalVariables|GetCurrent%20Token))
    (Math|Integer|IncrementInt (LocalVariables|GetCount)
      (:%20%20
        (bind _token_2 (CallFunction|GetTokenatPosition _column_adjusted _row_adjusted))
        (LocalVariables|SetCurrent%20Token _token_2))))
  (return (LocalVariables|GetCount)))