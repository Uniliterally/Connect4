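; C4Controller is the player controller for a turn-based token-dropping board game, apparently Connect Four.
; On BeginPlay, the local controller creates the Board widget, shows it and enables the mouse cursor with game-and-UI input.
; Its PlacePiece event takes a column number and, only when the player state's assigned token matches the game state's current turn, asks C4GameState to add that token to the column.
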(event Custom|Place%20Piece
  (params (Column%20Number :type Integer))
  (bind _asc4game_state (Utilities|Casting|CastToC4GameState (Game|GetGameState)))
  (bind _asc4player_state (Utilities|Casting|CastToC4PlayerState (Variables|GetPlayerState)))
  (if (Utilities|Enum|Equal(Enum) (Variables|/Game/Blueprints/Gameplay/C4PlayerState.C4PlayerState_C|GetAssigned%20Token _asc4player_state) (Variables|/Game/Blueprints/Gameplay/C4GameState.C4GameState_C|GetCurrent%20Turn _asc4game_state))
    (Default|AddTokentoColumn _asc4game_state Column%20Number (Variables|/Game/Blueprints/Gameplay/C4PlayerState.C4PlayerState_C|GetAssigned%20Token _asc4player_state))))

(event EventBeginPlay
  (if (Pawn|IsLocalPlayerController)
    (bind _returnvalue (UserInterface|CreateWidget "/Game/Blueprints/UI/Board.Board_C"))
    (bind _output_get (Variables|Default|SetBoardUI _returnvalue))
    (UserInterface|Viewport|AddtoViewport _output_get 0)
    (Input|SetInputModeGameandUI self _output_get "DoNotLock" true)
    (Variables|Default|SetbShowMouseCursor true)))

(fn ConstructionScript)